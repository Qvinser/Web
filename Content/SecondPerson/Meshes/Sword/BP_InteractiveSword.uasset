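; Interactive sword pickup that the player character can collect.
; A sphere trigger shows the Interact component when a MainCharacter begins overlapping and hides it when the overlap ends.
; On interact, it casts the character to BP_male_character, calls PickSword on it and destroys itself, leaving the pickup logic to the character.
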(event OnComponentBeginOverlap(Sphere)
  (params (OverlappedComponent :type Primitive%20Component%20Object%20Reference) (OtherActor :type Actor%20Object%20Reference) (OtherComp :type Primitive%20Component%20Object%20Reference) (OtherBodyIndex :type Integer) (bFromSweep :type Boolean) (SweepResult :type Hit%20Result%20Structure%20%28by%20ref%29))
  (Utilities|Casting|CastToMainCharacter OtherActor)
  (Rendering|SetVisibility (Variables|Default|GetInteract) true false))

(event OnComponentEndOverlap(Sphere)
  (params (OverlappedComponent :type Primitive%20Component%20Object%20Reference) (OtherActor :type Actor%20Object%20Reference) (OtherComp :type Primitive%20Component%20Object%20Reference) (OtherBodyIndex :type Integer))
  (Utilities|Casting|CastToMainCharacter OtherActor)
  (Rendering|SetVisibility (Variables|Default|GetInteract) false false))

(event EventBeginPlay
  (|CallParentFunction))

(event Collision|EventActorBeginOverlap
  (params (OtherActor :type Actor%20Object%20Reference))
  (|CallParentFunction OtherActor))

(event EventTick
  (params (DeltaSeconds :type Float%20%28single-precision%29))
  (|CallParentFunction 0.0))

(event EventOnInteract
  (params (Character :type Main%20Character%20Object%20Reference))
  (bind _asbp_male_character (Utilities|Casting|CastToBP_male_character Character))
  (Default|PickSword _asbp_male_character)
  (Actor|DestroyActor))

(fn ConstructionScript
  (|CallParentFunction))