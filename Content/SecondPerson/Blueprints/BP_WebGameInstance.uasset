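; BP_WebGameInstance is a game instance that forces Epic graphics quality when the game starts.
; On Init, it sets the overall scalability level, full resolution scale and individual quality groups such as textures, shadows, global illumination and effects through GameUserSettings.
; It then applies the settings without checking for command-line overrides, with no branch for platform or previously saved preferences.
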(event EventInit
  (bind _returnvalue (Settings|GetGameUserSettings))
  ;[1 1 1] 3 = Epic
  (Class|GameUserSettings|SetOverallScalabilityLevel _returnvalue 3)
  (Class|GameUserSettings|SetResolutionScaleValueEx _returnvalue 1e+02)
  (Class|GameUserSettings|SetTextureQuality _returnvalue 3)
  (Class|GameUserSettings|SetViewDistanceQuality _returnvalue 3)
  (Class|GameUserSettings|SetAntiAliasingQuality _returnvalue 3)
  (Class|GameUserSettings|SetShadowQuality _returnvalue 3)
  (Class|GameUserSettings|SetGlobalIlluminationQuality _returnvalue 3)
  (Class|GameUserSettings|SetReflectionQuality _returnvalue 3)
  (Class|GameUserSettings|SetVisualEffectQuality _returnvalue 3)
  (Class|GameUserSettings|SetFoliageQuality _returnvalue 3)
  (Class|GameUserSettings|SetShadowQuality _returnvalue 3)
  (Class|GameUserSettings|ApplySettings _returnvalue false))