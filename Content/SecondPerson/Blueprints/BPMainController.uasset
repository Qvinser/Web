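; BPMainController is a player controller that manages the in-game menu for the SecondPerson game.
; On BeginPlay it creates the GameMenu widget, adds it to the viewport and collapses it.
; The ShowMenu input action uses a FlipFlop to alternate between showing the menu with the mouse cursor and hiding both.
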(event EventBeginPlay
  (bind _returnvalue (UserInterface|CreateWidget "/Game/UI/GameMenu.GameMenu_C" self))
  (bind _output_get (Variables|Default|SetGameMenu _returnvalue))
  (UserInterface|Viewport|AddtoViewport _output_get 0)
  (Widget|SetVisibility _output_get "Collapsed"))

(event EventTick
  (params (DeltaSeconds :type Float%20%28single-precision%29)))

(event Input|ActionEvents|InputActionShowMenu
  (params (Key :type Key%20Structure :default "None"))
  (bind _gamemenu (Variables|Default|GetGameMenu))
  (:Pressed
    (Utilities|FlowControl|FlipFlop
      (:A
        (Widget|SetVisibility _gamemenu "Visible")
        (Variables|Default|SetbShowMouseCursor true))
      (:B
        (Widget|SetVisibility _gamemenu "Collapsed")
        (Variables|Default|SetbShowMouseCursor false)))))

(fn ConstructionScript)