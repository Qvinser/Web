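; Player character with sword melee combat, interaction and health shown on a HUD bar.
; Interact triggers the first overlapping BP_InteractiveActor, while PickSword adds a sword mesh to the right-hand socket and enables attacking.
; Left-click on the ground slows movement and briefly opens the sword's overlap window to damage characters.
; AnyDamage updates clamped health and the bar, treating negative damage as healing.
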(event Custom|PickSword
  (bind _returnvalue (AddComponent|AddSkeletalMeshComponent true (Variables|Default|GetRelative%20Transform)))
  (bind _output_get (Variables|Default|SetSword _returnvalue))
  (Components|SkeletalMesh|SetSkeletalMeshAsset _output_get "/Game/SecondPerson/Meshes/Sword/sword.sword")
  (Transformation|AttachComponentToComponent _returnvalue (Variables|Character|GetMesh) "CC_Base_R_HandSocket" "KeepRelative" "KeepRelative" "KeepRelative" true)
  (Variables|Default|SetHasWeapon true)
  (Variables|/Script/Engine.PrimitiveComponent|SetbGenerateOverlapEvents _returnvalue false)
  (Collision|SetCollisionEnabled _returnvalue "QueryAndPhysics")
  (Collision|AssignOnComponentBeginOverlap _returnvalue (delegate Custom|Overlp)))

(event Custom|Overlp
  (params (OverlappedComponent :type Primitive%20Component%20Object%20Reference) (OtherActor :type Actor%20Object%20Reference) (OtherComp :type Primitive%20Component%20Object%20Reference) (OtherBodyIndex :type Integer) (bFromSweep :type Boolean) (SweepResult :type Hit%20Result%20Structure%20%28by%20ref%29))
  (if (Variables|Default|GetIsAttacking)
    (bind _ascharacter (Utilities|Casting|CastToCharacter OtherActor))
    (Game|Damage|ApplyDamage _ascharacter 1e+01 0 0)))

(event EventBeginPlay
  (bind _asplayer_controller (Utilities|Casting|CastToPlayerController (Pawn|GetController)))
  (bind _returnvalue (UserInterface|CreateWidget "/Game/UI/HealthBar.HealthBar_C" _asplayer_controller))
  (bind _output_get (Variables|Default|SetHealthBar _returnvalue))
  (Default|UpdateBar _output_get 1.0)
  (UserInterface|Viewport|AddtoViewport _returnvalue 0))

(event Collision|EventActorBeginOverlap
  (params (OtherActor :type Actor%20Object%20Reference)))

(event EventTick
  (params (DeltaSeconds :type Float%20%28single-precision%29)))

(event Game|Damage|EventAnyDamage
  (params (Damage :type Float%20%28single-precision%29) (DamageType :type Damage%20Type%20Object%20Reference) (InstigatedBy :type Controller%20Object%20Reference) (DamageCauser :type Actor%20Object%20Reference))
  (if (> Damage 0.0)
    (bind _output_get (Variables|Default|SetHealth (Math|Float|Max(Float) (- (Variables|Default|GetHealth) Damage) 0.0)))
    (Default|UpdateBar (Variables|Default|GetHealthBar) (/ _output_get 1e+02))
    (else
      (bind _output_get_2 (Variables|Default|SetHealth (Math|Float|Min(Float) (- (Variables|Default|GetHealth) Damage) 1e+02)))
      (Default|UpdateBar (Variables|Default|GetHealthBar) (/ _output_get_2 1e+02)))))

(event Input|ActionEvents|InputActionInteract
  (params (Key :type Key%20Structure :default "None"))
  (:Released
    (bind _outactors (Collision|ComponentOverlapActors (Variables|Character|GetMesh) (Math|Conversions|ToTransform(Vector) (Transformation|GetActorLocation)) (Variables|Default|GetObject%20Types) 0))
    (bind _array_element (Utilities|Array|ForEachLoopwithBreak _outactors :!label _label)
      (:LoopBody
        (bind _asbp_interactive_actor (Utilities|Casting|CastToBP_InteractiveActor _array_element))
        (Default|OnInteract _asbp_interactive_actor self)
        (goto _label Break)))))

(event Input|MouseEvents|LeftMouseButton
  (params (Key :type Key%20Structure :default "None"))
  (:Pressed
    (if (and (and (Variables|Default|GetHasWeapon) (not (Variables|Default|GetIsAttacking))) (not (AI|Components|NavMovement|IsFalling (Variables|Character|GetCharacterMovement))))
      (Utilities|FlowControl|Sequence
        (:then_0
          ;[1 1 1] Preparing
          (Variables|/Script/Engine.CharacterMovementComponent|SetMaxWalkSpeed (Variables|Character|GetCharacterMovement) 3e+02)
          (Variables|Default|SetIsAttacking true))
        (:then_1
          ;[1 1 1] Action
          (Utilities|FlowControl|Delay 0.2)
          (Variables|/Script/Engine.PrimitiveComponent|SetbGenerateOverlapEvents (Variables|Default|GetSword) true)
          (Utilities|FlowControl|Delay 0.3)
          (Variables|Default|SetIsAttacking false)
          (Variables|/Script/Engine.PrimitiveComponent|SetbGenerateOverlapEvents (Variables|Default|GetSword) false)
          (Variables|/Script/Engine.CharacterMovementComponent|SetMaxWalkSpeed (Variables|Character|GetCharacterMovement) 5e+02))))))

(fn ConstructionScript)