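; Spider enemy that spawns an AI_Spider controller on begin play, melees the main character and dies at zero health.
; Attack plays a sped-up animation and opens a short IsAttacking window, during which the attack collision's overlap applies damage, then returns to the Animation Blueprint if alive.
; Incoming damage lowers Health; death stops and unpossesses the AI, plays the death animation and destroys the actor after a delay.
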(event OnComponentBeginOverlap(AttackCollision)
  (params (OverlappedComponent :type Primitive%20Component%20Object%20Reference) (OtherActor :type Actor%20Object%20Reference) (OtherComp :type Primitive%20Component%20Object%20Reference) (OtherBodyIndex :type Integer) (bFromSweep :type Boolean) (SweepResult :type Hit%20Result%20Structure%20%28by%20ref%29))
  (if (Variables|Default|GetIsAttacking)
    (bind _asmain_character (Utilities|Casting|CastToMainCharacter OtherActor))
    (Game|Damage|ApplyDamage _asmain_character 1e+01 0 0)
    (Development|PrintString "Damage")))

(event Custom|Attack
  (CallFunction|AttackMulticast))

(event Custom|DeathEvent
  (bind _returnvalue (Pawn|GetController))
  (bind _returnvalue_2 (AI|GetAIController _returnvalue))
  (Utilities|IsValid _returnvalue_2
    (:Is%20Valid
      (AI|Navigation|StopMovement _returnvalue_2)
      (Pawn|UnPossess _returnvalue_2)
      (CallFunction|DeathMulticast))))

(event Custom|DeathMulticast
  (Variables|Default|SetHealth 0.0)
  (Components|Animation|PlayAnimation (Variables|Character|GetMesh) "/Game/SecondPerson/Blueprints/Enemies/Spider/Animations/Armature_die.Armature_die" false)
  (Utilities|FlowControl|Delay 2.0)
  (Actor|DestroyActor))

(event Custom|AttackMulticast
  (bind _mesh (Variables|Character|GetMesh))
  (Variables|Default|SetIsAttacking true)
  (Components|Animation|PlayAnimation _mesh "/Game/SecondPerson/Blueprints/Enemies/Spider/Animations/Armature_attack.Armature_attack" false)
  (Components|Timeline|SetPlayRate _mesh 3.0)
  (Utilities|FlowControl|Delay 0.5)
  (if (> (Variables|Default|GetHealth) 0.0)
    (Components|Animation|SetAnimationMode _mesh "AnimationBlueprint" false)
    (Variables|Default|SetIsAttacking false)))

(event EventBeginPlay
  (Variables|Default|SetAIControllerClass "/Game/SecondPerson/Blueprints/Enemies/Spider/AI_Spider.AI_Spider_C")
  (Pawn|SpawnDefaultController))

(event Collision|EventActorBeginOverlap
  (params (OtherActor :type Actor%20Object%20Reference)))

(event EventTick
  (params (DeltaSeconds :type Float%20%28single-precision%29)))

(event Game|Damage|EventAnyDamage
  (params (Damage :type Float%20%28single-precision%29) (DamageType :type Damage%20Type%20Object%20Reference) (InstigatedBy :type Controller%20Object%20Reference) (DamageCauser :type Actor%20Object%20Reference))
  (bind _output_get (Variables|Default|SetHealth (Math|Float|Max(Float) (- (Variables|Default|GetHealth) Damage) 0.0)))
  (if (<= _output_get 0.0)
    (CallFunction|DeathEvent)))

(fn ConstructionScript)